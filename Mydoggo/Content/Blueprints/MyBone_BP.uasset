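; MyBone_BP is a bone pickup actor that the player collects by pressing F while overlapping it.
; Overlap events toggle Tick, enabling it only for the player, and set PickUpTextVisibility on FirstPersonCharacter.
; Tick polls for F, sets DogeBones to 1 on MydoggoCharacter rather than incrementing it, then destroys the bone.
; The prompt and pickup cast player 0's pawn to different character classes.
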(event `self.ReceiveActorEndOverlap`
  (params (OtherActor :type "Actor Object Reference"))
  (`self.SetActorTickEnabled` false)
  (bind _asfirst_person_character (cast `/Game/FirstPersonCPP/Blueprints/FirstPersonCharacter` (`GameplayStatics.GetPlayerCharacter` 0)))
  (set `/Game/FirstPersonCPP/Blueprints/FirstPersonCharacter.PickUpTextVisibility` false _asfirst_person_character))

(event `self.ReceiveActorBeginOverlap`
  (params (OtherActor :type "Actor Object Reference"))
  (bind _returnvalue (`GameplayStatics.GetPlayerCharacter` 0))
  (`self.SetActorTickEnabled` (== OtherActor _returnvalue))
  (bind _asfirst_person_character (cast `/Game/FirstPersonCPP/Blueprints/FirstPersonCharacter` _returnvalue))
  (set `/Game/FirstPersonCPP/Blueprints/FirstPersonCharacter.PickUpTextVisibility` true _asfirst_person_character))

(event `self.ReceiveTick`
  (params (DeltaSeconds :type "Float (single-precision)"))
  (if (`PlayerController.WasInputKeyJustPressed` (`GameplayStatics.GetPlayerController` 0) "F")
    (bind _asmydoggo_character (cast `MydoggoCharacter` (`GameplayStatics.GetPlayerCharacter` 0)))
    (`MydoggoCharacter.SetDogeBones` _asmydoggo_character 1)
    (`self.K2_DestroyActor`)))

(fn `UserConstructionScript`)