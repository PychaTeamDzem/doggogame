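; Delivery trigger actor that visually marks listed delivery objects when they overlap it.
; On BeginPlay it caches the result of GetObjectTimeList in a temporary array.
; When a DeliveryObject_BP begins overlapping, it searches that array for the same actor and, on a match, swaps its root static mesh's first material to FootprintDecal_mat.
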(event `self.ReceiveBeginPlay`
  (bind _returnvalue (`self.GetObjectTimeList`))
  (set `self.TempObjectArray` _returnvalue))

(event `self.ReceiveActorBeginOverlap`
  (params (OtherActor :type "Actor Object Reference"))
  (if (== (`GameplayStatics.GetObjectClass` OtherActor) "/Game/Blueprints/DeliveryObject_BP.DeliveryObject_BP_C")
    (for _array_element (`self.TempObjectArray`)
      (if (== OtherActor _array_element)
        (bind _asstatic_mesh_component (cast `StaticMeshComponent` (`Actor.RootComponent` OtherActor)))
        (`PrimitiveComponent.SetMaterial` _asstatic_mesh_component 0 "/Game/misc/FootprintDecal_mat.FootprintDecal_mat")
        (break)))))

(fn `UserConstructionScript`)